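; HUD Blueprint for the Bloodstream HUD that provides a crosshair fixed in front of the player camera.
; On BeginPlay it spawns a CrosairActor a set distance along the camera's forward vector and attaches it to the camera manager.
; Each Tick projects the camera's forward vector onto the pawn's right and up axes, hiding the crosshair outside a horizontal and asymmetric vertical angle window.
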(event EventTick
  (params (DeltaSeconds :type Float%20%28single-precision%29))
  (bind _returnvalue (Game|GetPlayerCameraManager 0))
  (bind _returnvalue_2 (Game|Player|GetPlayerPawn 0))
  (bind _returnvalue_3 (Transformation|GetActorRotation _returnvalue_2))
  (bind _returnvalue_4 (Camera|GetCameraRotation _returnvalue))
  (bind _returnvalue_5 (Math|Vector|GetForwardVector _returnvalue_4))
  (bind _returnvalue_6 (Math|Vector|GetRightVector _returnvalue_3))
  (bind _returnvalue_7 (Math|Vector|GetUpVector _returnvalue_3))
  (bind _returnvalue_8 (Math|Vector|DotProduct _returnvalue_6 _returnvalue_5))
  (bind _returnvalue_9 (Math|Vector|DotProduct _returnvalue_5 _returnvalue_7))
  (bind _returnvalue_10 (Class|KismetMathLibrary|DegAsin _returnvalue_8))
  (bind _returnvalue_11 (Class|KismetMathLibrary|DegAsin _returnvalue_9))
  (bind _output_get (Variables|Default|SetIsHidden (not (Math|Boolean|ANDBoolean (>= _returnvalue_10 -34.0) (<= _returnvalue_10 34.0) (>= _returnvalue_11 -6e+01) (<= _returnvalue_11 23.0)))))
  (Default|SetHidden (Variables|Default|GetCrosshair) _output_get))

(event EventBeginPlay
  (bind _returnvalue (Game|GetPlayerCameraManager 0))
  (bind _returnvalue_2 (Transformation|GetActorLocation _returnvalue))
  (bind _returnvalue_3 (Transformation|GetActorForwardVector _returnvalue))
  (bind _returnvalue_4 (* _returnvalue_3 3e+02))
  (bind _returnvalue_5 (+ _returnvalue_2 _returnvalue_4))
  ;[1 1 1] Static Hud infront of Camera
  (Variables|Default|SetHUDRotation (Transformation|GetActorRotation _returnvalue))
  (Variables|Default|SetHUDLocation _returnvalue_5)
  (bind _returnvalue_6 (Game|SpawnActorfromClass "/Game/Blueprint/HUD/CrosairActor.CrosairActor_C" (Math|Conversions|ToTransform(Vector) _returnvalue_5) true 0))
  (bind _output_get (Variables|Default|SetCrosshair _returnvalue_6))
  (Class|Actor|AttachRootComponenttoActor _output_get (Game|GetPlayerCameraManager 0) "None" "KeepRelativeOffset" true))

(fn ConstructionScript)