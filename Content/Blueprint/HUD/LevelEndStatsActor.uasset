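; Actor that shows the level-end stats screen through a LevelEndStats widget component, hidden at BeginPlay.
; BeginPlay caches the widget's eight objective text boxes plus its title and subtitle, which events can update individually.
; ActivateLevelEndStats reveals the display and takes parallel bool and text arrays, listing only achieved entries packed from the first box.
; The achieved list is never cleared and is not capped at the eight boxes.
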(event Custom|setText
  (params (newText :type Text) (textboxIndex :type Integer :default 0))
  (Rendering|Components|TextRender|SetText (Utilities|Array|Get(acopy) (Variables|Default|Gettextboxes) textboxIndex) newText))

(event Custom|changetitle
  (params (NewText :type Text))
  (Rendering|Components|TextRender|SetText (Variables|Default|Gettitletext) NewText))

(event Custom|changeSubtitle
  (params (NewText :type Text))
  (Rendering|Components|TextRender|SetText (Variables|Default|Getsubtitletext) NewText))

(event EventBeginPlay
  (Rendering|SetVisibility false false)
  (bind _aslevel_end_stats (Utilities|Casting|CastToLevelEndStats (UserInterface|GetUserWidgetObject (Variables|Default|GetlevelendstatsWidget))))
  ;[1 1 1] Set textboxes and checkboxes array
  (Utilities|Array|SetArrayElem (Variables|Default|Gettextboxes) 0 (Variables|/Game/Blueprint/HUD/LevelEndStats.LevelEndStats_C|GetEditableText_objective1 _aslevel_end_stats) true)
  (Utilities|Array|SetArrayElem (Variables|Default|Gettextboxes) 1 (Variables|/Game/Blueprint/HUD/LevelEndStats.LevelEndStats_C|GetEditableText_objective2 _aslevel_end_stats) true)
  (Utilities|Array|SetArrayElem (Variables|Default|Gettextboxes) 2 (Variables|/Game/Blueprint/HUD/LevelEndStats.LevelEndStats_C|GetEditableText_objective3 _aslevel_end_stats) true)
  (Utilities|Array|SetArrayElem (Variables|Default|Gettextboxes) 3 (Variables|/Game/Blueprint/HUD/LevelEndStats.LevelEndStats_C|GetEditableText_objective4 _aslevel_end_stats) true)
  (Utilities|Array|SetArrayElem (Variables|Default|Gettextboxes) 4 (Variables|/Game/Blueprint/HUD/LevelEndStats.LevelEndStats_C|GetEditableText_objective5 _aslevel_end_stats) true)
  (Utilities|Array|SetArrayElem (Variables|Default|Gettextboxes) 5 (Variables|/Game/Blueprint/HUD/LevelEndStats.LevelEndStats_C|GetEditableText_objective6 _aslevel_end_stats) true)
  (Utilities|Array|SetArrayElem (Variables|Default|Gettextboxes) 6 (Variables|/Game/Blueprint/HUD/LevelEndStats.LevelEndStats_C|GetEditableText_objective7 _aslevel_end_stats) true)
  (Utilities|Array|SetArrayElem (Variables|Default|Gettextboxes) 7 (Variables|/Game/Blueprint/HUD/LevelEndStats.LevelEndStats_C|GetEditableText_objective8 _aslevel_end_stats) true)
  (Variables|Default|Settitletext (Variables|/Game/Blueprint/HUD/LevelEndStats.LevelEndStats_C|GetTitleText _aslevel_end_stats))
  (Variables|Default|Setsubtitletext (Variables|/Game/Blueprint/HUD/LevelEndStats.LevelEndStats_C|GetSubtitleText _aslevel_end_stats)))

(event EventActorBeginOverlap
  (params (OtherActor :type Actor%20Object%20Reference)))

(event EventTick
  (params (DeltaSeconds :type Float%20%28single-precision%29)))

(fn ConstructionScript)

(fn ActivateLevelEndStats
  (params (Achievement_Bools :type Array%20of%20Booleans) (Achievement_Texts :type Array%20of%20Texts))
  (LocalVariables|Setach_bools Achievement_Bools)
  (LocalVariables|Setach_texts Achievement_Texts)
  (Rendering|SetVisibility self true false)
  (for (_array_element _array_index) (LocalVariables|Getach_bools)
    (if _array_element
      (Utilities|Array|Add (LocalVariables|Getfin_achievements) (Utilities|Array|Get(acopy) (LocalVariables|Getach_texts) _array_index))))
  (for (_array_element_2 _array_index_2) (LocalVariables|Getfin_achievements)
    (Rendering|Components|TextRender|SetText (Utilities|Array|Get(acopy) (Variables|Default|Gettextboxes) _array_index_2) _array_element_2)))