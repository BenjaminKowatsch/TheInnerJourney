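; ObjectiveActor is an actor that exposes control over a three-slot objectives display shown through its ObjectiveWidget component.
; On BeginPlay it casts the component's user widget to Objectives and caches references to its three editable texts and three checkboxes.
; Per-slot custom events then set each objective's text and each checkbox's visibility and checked state.
; It holds no objective logic itself and only forwards values passed to those events.
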(event Custom|setText1
  (params (newText :type Text))
  (Rendering|Components|TextRender|SetText (Variables|Default|Gettext1) newText))

(event Custom|setVisibilityCheckbox1
  (params (visib :type ESlateVisibility%20Enum :default "Visible"))
  (Widget|SetVisibility (Variables|Default|Getbox1) visib))

(event Custom|setVisibilityCheckbox2
  (params (visib :type ESlateVisibility%20Enum :default "Visible"))
  (Widget|SetVisibility (Variables|Default|Getbox2) visib))

(event Custom|setVisibilityCheckbox3
  (params (visib :type ESlateVisibility%20Enum :default "Visible"))
  (Widget|SetVisibility (Variables|Default|Getbox3) visib))

(event Custom|setText2
  (params (NewText :type Text))
  (Rendering|Components|TextRender|SetText (Variables|Default|Gettext2) NewText))

(event Custom|setText3
  (params (New%20text :type Text))
  (Rendering|Components|TextRender|SetText (Variables|Default|Gettext3) New%20text))

(event Custom|setToggledCheckbox3
  (params (checked :type Boolean))
  (Class|CheckBox|SetIsChecked (Variables|Default|Getbox3) checked))

(event Custom|setToggledCheckbox1
  (params (checked :type Boolean))
  (Class|CheckBox|SetIsChecked (Variables|Default|Getbox1) checked))

(event Custom|setToggledCheckbox2
  (params (checked :type Boolean))
  (Class|CheckBox|SetIsChecked (Variables|Default|Getbox2) checked))

(event EventBeginPlay
  (bind _asobjectives (Utilities|Casting|CastToObjectives (UserInterface|GetUserWidgetObject (Variables|Default|GetobjectiveWidget))))
  (Variables|Default|Settext1 (Variables|/Game/Blueprint/HUD/Objectives.Objectives_C|GetEditableText_objective1 _asobjectives))
  (Variables|Default|Settext2 (Variables|/Game/Blueprint/HUD/Objectives.Objectives_C|GetEditableText_objective2 _asobjectives))
  (Variables|Default|Settext3 (Variables|/Game/Blueprint/HUD/Objectives.Objectives_C|GetEditableText_objective3 _asobjectives))
  (Variables|Default|Setbox1 (Variables|/Game/Blueprint/HUD/Objectives.Objectives_C|GetCheckBox_1 _asobjectives))
  (Variables|Default|Setbox2 (Variables|/Game/Blueprint/HUD/Objectives.Objectives_C|GetCheckBox_2 _asobjectives))
  (Variables|Default|Setbox3 (Variables|/Game/Blueprint/HUD/Objectives.Objectives_C|GetCheckBox_3 _asobjectives)))

(event EventActorBeginOverlap
  (params (OtherActor :type Actor%20Object%20Reference)))

(event EventTick
  (params (DeltaSeconds :type Float%20%28single-precision%29)))

(fn ConstructionScript)