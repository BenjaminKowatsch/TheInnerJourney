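; Croshair_Hud places a world-space crosshair in front of the player's view.
; On BeginPlay it spawns a CrosairActor 300 units along the player camera manager's forward vector, using a location-only transform.
; It then attaches that actor to the camera manager so it follows the camera, with no per-tick update.
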(event EventBeginPlay
  (Variables|Default|SetCamera (Game|GetPlayerCameraManager 0))
  (Variables|Default|SetHUDRotation (Transformation|GetActorRotation (Variables|Default|GetCamera)))
  (Variables|Default|SetHUDLocation (+ (Transformation|GetActorLocation (Variables|Default|GetCamera)) (* (Math|Vector|GetForwardVector (Variables|Default|GetHUDRotation)) 3e+02)))
  (bind _returnvalue (Game|SpawnActorfromClass "/Game/Blueprint/FreeFlight/CrosairActor.CrosairActor_C" (Math|Conversions|ToTransform(Vector) (+ (Transformation|GetActorLocation (Variables|Default|GetCamera)) (* (Math|Vector|GetForwardVector (Variables|Default|GetHUDRotation)) 3e+02))) true 0))
  (Class|Actor|AttachRootComponenttoActor _returnvalue (Variables|Default|GetCamera) "None" "KeepRelativeOffset" true))

(fn ConstructionScript)