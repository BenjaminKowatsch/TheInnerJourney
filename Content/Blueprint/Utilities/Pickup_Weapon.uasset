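; Weapon power-up pickup that floats and spins until a ship collects it.
; A looping-style idle animation comes from a timeline started on BeginPlay, which adds bob offsets on all three axes and yaw rotation each update.
; A randomized timeline start position varies the motion between instances.
; Overlap of the THelferzelleTextured component by Ship_BP increments that ship's power-up counter and destroys the pickup.
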(event OnComponentBeginOverlap(T-HelferzelleTextured)
  (params (OtherActor :type Actor%20Object%20Reference) (OtherComp :type Primitive%20Component%20Object%20Reference) (OtherBodyIndex :type Integer) (bFromSweep :type Boolean) (SweepResult :type Hit%20Result%20Structure%20%28by%20ref%29))
  (bind _asship_bp (Utilities|Casting|CastToShip_BP OtherActor))
  (Default|IncreasePowerUpCounter _asship_bp)
  (Actor|DestroyActor)
  (bind (_direction _rotation _float_bob) (Timeline|Timeline_0 Stop)
    (:Update
      (Transformation|AddRelativeLocation (Math|Vector|MakeVector _float_bob _float_bob _float_bob) false)
      (Transformation|AddRelativeRotation (Class|KismetMathLibrary|MakeRot 0.0 _rotation 0.0) false))))

(event EventBeginPlay
  (Components|Timeline|SetPlaybackPosition (Variables|Default|GetTimeline_0) (Math|Random|RandomFloatinRange 0.0 5.0) false)
  (bind (_direction _rotation _float_bob) (Timeline|Timeline_0 Play)
    (:Update
      (Transformation|AddRelativeLocation (Math|Vector|MakeVector _float_bob _float_bob _float_bob) false)
      (Transformation|AddRelativeRotation (Class|KismetMathLibrary|MakeRot 0.0 _rotation 0.0) false))))

(fn ConstructionScript)