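; Health pickup actor that heals a Ship_BP on overlap and then destroys itself.
; A timeline, started at a random position on BeginPlay, rotates and bobs the pickup through relative offsets on each update.
; The orb mesh's overlap event casts the other actor to Ship_BP and passes HealValue to Heal.
; The SelfDistruct option only triggers a delay, with nothing wired after it.
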(event OnComponentBeginOverlap(HealthOrb_lod0)
  (params (OtherActor :type Actor%20Object%20Reference) (OtherComp :type Primitive%20Component%20Object%20Reference) (OtherBodyIndex :type Integer) (bFromSweep :type Boolean) (SweepResult :type Hit%20Result%20Structure%20%28by%20ref%29))
  (bind _asship_bp (Utilities|Casting|CastToShip_BP OtherActor))
  (Default|Heal _asship_bp (Variables|Default|GetHeal%20Value))
  (Actor|DestroyActor))

(event EventBeginPlay
  (Components|Timeline|SetPlaybackPosition (Variables|Default|GetAnim) (Math|Random|RandomFloatinRange 0.0 5.0) false)
  (bind (_direction _rotation _float_bob) (Timeline|Anim Play)
    (:Update
      (Transformation|AddRelativeRotation (Class|KismetMathLibrary|MakeRot 0.0 _rotation 0.0) false)
      (Transformation|AddRelativeLocation (Math|Vector|MakeVector 0.0 0.0 _float_bob) false)
      (if (Variables|Default|GetSelf%20Distruct)
        (Utilities|FlowControl|Delay (Variables|Default|GetDestruction%20Delay))))))

(fn ConstructionScript)