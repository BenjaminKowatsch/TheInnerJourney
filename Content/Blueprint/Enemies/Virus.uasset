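; Virus enemy that damages the player's ship on contact and can be destroyed for a chance at a pickup.
; A timeline, started at a random position to vary instances, drives its spin, bob and scale pulse.
; Depleted health triggers a sound and destruction, then rolls for a health pickup, falling back to a weapon pickup roll.
; Overlapping the ship plays a sound, disables collision, applies damage and runs a resize timeline before destroying itself.
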(event OnComponentBeginOverlap(Box)
  (params (OtherActor :type Actor%20Object%20Reference) (OtherComp :type Primitive%20Component%20Object%20Reference) (OtherBodyIndex :type Integer) (bFromSweep :type Boolean) (SweepResult :type Hit%20Result%20Structure%20%28by%20ref%29))
  (bind _asship_bp (Utilities|Casting|CastToShip_BP OtherActor))
  (Audio|PlaySoundatLocation 0 (Transformation|GetWorldLocation)) ; Sound Virus Collided with Ship
  (Collision|SetActorEnableCollision false)
  (Game|Damage|ApplyDamage _asship_bp (Variables|Default|GetDamage) 0 0)
  (bind _resize (Timeline|Resize Play)
    (:Update
      (Transformation|SetActorRelativeScale3D (Math|Conversions|ToVector(Float) _resize)))
    (:Finished
      (Actor|DestroyActor))))

(event EventBeginPlay
  (Components|Timeline|SetPlaybackPosition (Variables|Default|GetAnimation) (Math|Random|RandomFloatinRange 0.0 5.0) false)
  (bind (_direction _rotation _float_bob _resize) (Timeline|Animation Play)
    (:Update
      (Transformation|AddRelativeRotation (Class|KismetMathLibrary|MakeRot 0.0 _rotation 0.0) false)
      (Transformation|AddRelativeLocation (Math|Vector|MakeVector _float_bob _float_bob _float_bob) false)
      (Transformation|AddRelativeLocation (Math|Vector|MakeVector _float_bob _float_bob _float_bob) false)
      (Transformation|SetActorRelativeScale3D (Math|Conversions|ToVector(Float) _resize)))))

(event EventAnyDamage
  (params (Damage :type Float%20%28single-precision%29) (DamageType :type Damage%20Type%20Object%20Reference) (InstigatedBy :type Controller%20Object%20Reference) (DamageCauser :type Actor%20Object%20Reference))
  (bind _returnvalue (Transformation|GetWorldLocation))
  ;[1 1 1] Recieve Damage
  (bind _output_get (Variables|Default|SetHealth (- (Variables|Default|GetHealth) Damage)))
  (if (< _output_get 0.0)
    (Variables|Default|SetLocation _returnvalue)
    (Audio|PlaySoundatLocation 0 _returnvalue) ; Destroyed With Weapon Sound
    (Actor|DestroyActor)
    (if (<= (Math|Random|RandomFloat) (Variables|Default|GetHealthPickupProbability))
      ;[1 1 1] Spawn Health
      (bind _returnvalue_2 (Game|SpawnActorfromClass "/Game/Blueprint/Utilities/Health_Pickup.Health_Pickup_C" (Math|Transform|MakeTransform (Variables|Default|GetLocation) (Transformation|GetActorRotation)) false 0))
      (Transformation|SetActorScale3D _returnvalue_2 "5.000000,5.000000,5.000000")
      (else
        ;[1 1 1] Spawn Weapon Pickup
        (if (<= (Math|Random|RandomFloat) (Variables|Default|GetT-Helper%20Probability))
          (bind _returnvalue_3 (Game|SpawnActorfromClass "/Game/Blueprint/Utilities/Pickup_Weapon.Pickup_Weapon_C" (Math|Transform|MakeTransform (Variables|Default|GetLocation) (Transformation|GetActorRotation)) false 0))
          (Transformation|SetActorScale3D _returnvalue_3 "40.000000,40.000000,40.000000"))))))

(fn ConstructionScript)