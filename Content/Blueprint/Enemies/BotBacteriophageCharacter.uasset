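; Flying bacteriophage enemy character that poisons the player's Ship_BP while it is inside the PoisonRadius and eventually explodes.
; Tick eases the actor toward a tilted rotation and runs PoisonTick, which applies periodic damage on overlap.
; Accumulated exposure triggers a final damage burst, a poison particle effect and self-destruction.
; AddWaypoint collects unique waypoints and writes a randomly chosen one, with its index, to the AI Blackboard.
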(event OnComponentBeginOverlap(PoisonRadius)
  (params (OtherActor :type Actor%20Object%20Reference) (OtherComp :type Primitive%20Component%20Object%20Reference) (OtherBodyIndex :type Integer) (bFromSweep :type Boolean) (SweepResult :type Hit%20Result%20Structure%20%28by%20ref%29))
  ;[1 1 1] Damage Logic
  (bind _asship_bp (Utilities|Casting|CastToShip_BP OtherActor))
  (Variables|Default|SetPoison%20Time true))

(event OnComponentEndOverlap(PoisonRadius)
  (params (OtherActor :type Actor%20Object%20Reference) (OtherComp :type Primitive%20Component%20Object%20Reference) (OtherBodyIndex :type Integer))
  ;[1 1 1] Damage Logic
  (Utilities|Casting|CastToShip_BP OtherActor)
  (Variables|Default|SetPoison%20Time false))

(event Custom|Poison%20Tick
  (bind _returnvalue (Utilities|Time|GetWorldDeltaSeconds))
  ;[1 1 1] Damage Logic
  (if (Variables|Default|GetPoison%20Time)
    (bind _output_get (Variables|Default|SetPoisonTime (+ _returnvalue (Variables|Default|GetPoisonTime))))
    (Variables|Default|SetExplosionTime (+ _returnvalue (Variables|Default|GetExplosionTime)))
    (if (> _output_get (Variables|Damage|GetPoisonTimeTillDamage))
      (if (> (Variables|Default|GetExplosionTime) (Variables|Damage|GetTime%20till%20Explosion))
        (Game|Damage|ApplyDamage (stale OnComponentBeginOverlap(PoisonRadius) _asship_bp) 25.0 0 0)
        (Actor|DestroyActor)
        (Effects|SpawnEmitteratLocation "/Game/Particles/BloodStream/P_Poison2.P_Poison2" (Transformation|GetActorLocation))
        (else
          (Variables|Default|SetPoisonTime 0.0)
          (Game|Damage|ApplyDamage (stale OnComponentBeginOverlap(PoisonRadius) _asship_bp) (Variables|Damage|GetPoison%20Damage) 0 0))))))

(event EventTick
  (params (DeltaSeconds :type Float%20%28single-precision%29))
  ;[1 1 1] Gameloop
  (Transformation|SetActorRotation (Math|Interpolation|RInterpTo (Transformation|GetActorRotation) (Math|Vector|RotatorfromAxisandAngle (Math|Vector|RotateVector (Math|Vector|GetRightVector "0, 0, 0") (Variables|Default|GetRotation)) (Variables|Default|GetTiltAngle)) DeltaSeconds 1.0))
  (CallFunction|PoisonTick))

(event EventBeginPlay
  ;[1 1 1] Initialize
  (Variables|/Script/Engine.CharacterMovementComponent|SetMaxFlySpeed (Variables|Character|GetCharacterMovement) (* (Variables|Default|GetMovementSpeed) (Variables|Default|GetSpeedRate))))

(fn ConstructionScript)

(fn AddWaypoint
  (params (Waypoint :type Bot%20Bacteriophage%20Waypoint%20Object%20Reference))
  (bind _returnvalue (AI|GetBlackboard 0))
  (bind _waypoints (Variables|Default|GetWaypoints))
  (bind _returnvalue_2 (Utilities|Array|AddUnique _waypoints Waypoint))
  (if (not (< _returnvalue_2 0))
    (bind _output_get (LocalVariables|SetRandomIndex (Math|Random|RandomInteger (Utilities|Array|Length _waypoints))))
    (AI|Components|Blackboard|SetValueasObject _returnvalue (Utilities|Name|MakeLiteralName "CurrentWaypoint") (Utilities|Array|Get(acopy) _waypoints _output_get))
    (Class|BlackboardComponent|SetValueasInt _returnvalue (Utilities|Name|MakeLiteralName "CurrentWaypointIndex") _output_get)))