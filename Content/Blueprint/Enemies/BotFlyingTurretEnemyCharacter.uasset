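; Flying turret enemy character that fires projectiles on a repeating interval, with aiming and firing each toggled by a flag.
; Tick recomputes the projectile rotation toward the LookAt position without turning the actor, then calls Fire.
; Fire relies on Delay ignoring re-triggers to throttle per-tick calls.
; It spawns the weapon projectile offset along the actor's up vector, using that rotation, even if colliding.
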(event Custom|Update%20Rotation
  ;[1 1 1] Update Rotation Event
  (if (Variables|Default|GetRotateEnabled)
    (Variables|Default|SetProjectileRotation (Math|Rotator|FindLookatRotation (Transformation|GetActorLocation) (Variables|Default|GetLookAt)))))

(event Custom|Fire
  ;[1 1 1] Fire Event
  (if (Variables|Default|GetFireEnabled)
    (Utilities|FlowControl|Delay (Variables|Default|GetFireInterval))
    (Game|SpawnActorfromClass "/Game/Blueprint/Weapons/Weapon_Projectile.Weapon_Projectile_C" (Math|Transform|MakeTransform (+ (Transformation|GetActorLocation) (* (Math|Vector|GetUpVector (Transformation|GetActorRotation)) (Variables|Default|GetBulletSpawnDistance))) (Variables|Default|GetProjectileRotation)) true 0)))

(event EventTick
  (params (DeltaSeconds :type Float%20%28single-precision%29))
  ;[1 1 1] GameLoop
  (|CallParentFunction DeltaSeconds)
  (CallFunction|UpdateRotation)
  (CallFunction|Fire))

(fn ConstructionScript
  (|CallParentFunction))