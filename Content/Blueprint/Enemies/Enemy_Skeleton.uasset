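; Skeleton enemy that tracks damage and can drop pickups when it dies.
; AnyDamage only subtracts from Health; a separate ShrinkToDeath event runs a timeline that repeatedly multiplies the actor's scale by its track value.
; When the timeline finishes, random rolls spawn a health pickup or, failing that, possibly a weapon pickup.
; The actor is destroyed only on the branches where a pickup spawns.
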(event Custom|ShrinkToDeath
  (bind _returnvalue (Transformation|GetActorLocation))
  (bind _returnvalue_2 (Transformation|GetActorRotation))
  (bind _newtrack_0 (Timeline|Timeline_0 Play)
    (:Update
      (Transformation|SetWorldScale3D (* (Transformation|GetWorldScale) _newtrack_0)))
    (:Finished
      (Development|PrintString "Hello")
      (if (<= (Math|Random|RandomFloat) (Variables|Default|GetHealthPickupSpawnProbability))
        (Game|SpawnActorfromClass "/Game/Blueprint/Utilities/Health_Pickup.Health_Pickup_C" (Math|Transform|MakeTransform _returnvalue _returnvalue_2 "5.000000,5.000000,5.000000") true 0)
        (Actor|DestroyActor :!label _label)
        (elif (<= (Math|Random|RandomFloat) (Variables|Default|GetT-HelperSpawnProbability))
          (Game|SpawnActorfromClass "/Game/Blueprint/Utilities/Pickup_Weapon.Pickup_Weapon_C" (Math|Transform|MakeTransform _returnvalue _returnvalue_2 "30.000000,30.000000,30.000000") true 0)
          (goto _label))))))

(event EventAnyDamage
  (params (Damage :type Float%20%28single-precision%29) (DamageType :type Damage%20Type%20Object%20Reference) (InstigatedBy :type Controller%20Object%20Reference) (DamageCauser :type Actor%20Object%20Reference))
  ;[1 1 1] Recieve Damage
  (Variables|Default|SetHealth (- (Variables|Default|GetHealth) Damage)))

(fn ConstructionScript)