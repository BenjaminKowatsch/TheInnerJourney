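; Turret enemy character that turns toward a LookAt target and fires projectiles, with a brain variant event that swaps material and scales it up.
; Tick smoothly interpolates actor yaw to the target while storing the unsmoothed, unclamped aim as BarrelRotation.
; Tick also drives firing, using a Delay as the interval gate.
; Projectiles spawn with BarrelRotation, offset along its up vector, so the clamped pitch never affects them.
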(event Custom|Update%20Rotation
  (bind _returnvalue (Transformation|GetActorLocation))
  (bind _lookat (Variables|TurretSettings|GetLookAt))
  (bind _returnvalue_2 (Math|Rotator|FindLookatRotation _returnvalue _lookat))
  (bind (_pitch _yaw) (Class|KismetMathLibrary|BreakRot _returnvalue_2))
  ;[1 1 1] Update Rotation Event
  (if (Variables|TurretSettings|GetRotateEnabled)
    (Variables|TurretSettings|SetBarrelRotation _returnvalue_2)
    (Transformation|SetActorRotation (Class|KismetMathLibrary|MakeRot 0.0 (.Yaw (Class|KismetMathLibrary|BreakRot (Math|Interpolation|RInterpTo (Transformation|GetActorRotation) (Class|KismetMathLibrary|MakeRot (Math|Float|ClampAngle _pitch (Variables|TurretSettings|GetMinAngle) (Variables|TurretSettings|GetMaxAngle)) _yaw 0.0) (Utilities|Time|GetWorldDeltaSeconds) (Variables|TurretSettings|GetRotationSpeed)))) 0.0))))

(event Custom|Fire
  (bind _barrelrotation (Variables|TurretSettings|GetBarrelRotation))
  ;[1 1 1] Fire Event
  (if (Variables|TurretSettings|GetFireEnabled)
    (Utilities|FlowControl|Delay (Variables|TurretSettings|GetFireInterval))
    (Game|SpawnActorfromClass "/Game/Blueprint/Weapons/Weapon_Projectile.Weapon_Projectile_C" (Math|Transform|MakeTransform (+ (Transformation|GetActorLocation) (* (Math|Vector|GetUpVector _barrelrotation) (Variables|TurretSettings|GetProjectileSpawnDistance))) _barrelrotation) false 0)))

(event Custom|MakeBrainEnemy
  (Rendering|Material|SetMaterial 0 "/Game/Materials/Enemies/TurretBrain.TurretBrain")
  (Transformation|SetActorRelativeScale3D "10.000000,10.000000,10.000000"))

(event EventTick
  (params (DeltaSeconds :type Float%20%28single-precision%29))
  ;[1 1 1] GameLoop
  (CallFunction|UpdateRotation)
  (CallFunction|Fire))

(fn ConstructionScript)