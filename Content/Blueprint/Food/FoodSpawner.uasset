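; FoodSpawner populates the level with food actors once at BeginPlay.
; It spawns one moving pizza at one of the first two PizzaSpawnpoint actors, chosen randomly, and passes it a rotation intensity.
; It then shuffles FoodClasses and spawns one food per FoodSpawnpoint by matching array index.
; Each Food_moving gets a random start delay and movement factor to vary its breathing motion.
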(event EventBeginPlay
  (CallFunction|SpawnPizza)
  (CallFunction|SpawnFoods))

(event EventActorBeginOverlap
  (params (OtherActor :type Actor%20Object%20Reference)))

(event EventTick
  (params (DeltaSeconds :type Float%20%28single-precision%29)))

(fn ConstructionScript)

(fn SpawnPizza
  (bind _outactors (Actor|GetAllActorsOfClass "/Game/Blueprint/Food/PizzaSpawnpoint.PizzaSpawnpoint_C"))
  (bind _output_get (Variables|Default|SetPizza_Spawnpoints _outactors))
  (bind _returnvalue (Game|SpawnActorfromClass "/Game/Blueprint/Food/Food_moving_Pizza.Food_moving_Pizza_C" (Transformation|GetActorTransform (Utilities|Array|Get(acopy) _output_get (Math|Random|RandomInteger 2))) true 0))
  (bind _asfood_moving_pizza (Utilities|Casting|CastToFood_moving_Pizza _returnvalue)
    (:then
      (Variables|/Game/Blueprint/Food/Food_moving_Pizza.Food_moving_Pizza_C|SetRotaionIntensity _asfood_moving_pizza (Variables|Default|GetPizzaRotationIntensity)))
    (:CastFailed
      _))
  (return))

(fn SpawnFoods
  (bind _foodclasses (Variables|Default|GetFoodClasses))
  ;[1 1 1] Iterate over Spawnpoints
  (bind _outactors (Actor|GetAllActorsOfClass "/Game/Blueprint/Food/FoodSpawnpoint.FoodSpawnpoint_C"))
  (bind _output_get (Variables|Default|SetFood_Spawnpoints _outactors))
  (Utilities|Array|Shuffle _foodclasses)
  (for (_array_element _array_index) _output_get
    ;[1 1 1] Spawn Actor at Spawnpoint
    (bind _returnvalue (Game|SpawnActorfromClass (Utilities|Array|Get(acopy) _foodclasses _array_index) (Transformation|GetActorTransform _array_element) true 0))
    ;[1 1 1] Randomize breathing intensity
    (bind _asfood_moving (Utilities|Casting|CastToFood_moving _returnvalue))
    (Variables|/Game/Blueprint/Food/Food_moving.Food_moving_C|SetStartDelay _asfood_moving (Math|Random|RandomFloatinRange 0.0 2.0))
    (Variables|/Game/Blueprint/Food/Food_moving.Food_moving_C|SetMovementFactor _asfood_moving (Math|Random|RandomFloatinRange 0.5 2.5)))
  (return))