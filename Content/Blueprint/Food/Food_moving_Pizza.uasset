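; Moving pizza food Blueprint that spins and triggers the pizza achievement when the player's ship touches it.
; Tick runs the parent logic, then adds a roll rotation of RotaionIntensity each frame, not scaled by delta time.
; The Box component's begin overlap casts the other actor to Ship_BP and, on success, calls CallPizzaAchievement.
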(event OnComponentBeginOverlap(Box)
  (params (OtherActor :type Actor%20Object%20Reference) (OtherComp :type Primitive%20Component%20Object%20Reference) (OtherBodyIndex :type Integer) (bFromSweep :type Boolean) (SweepResult :type Hit%20Result%20Structure%20%28by%20ref%29))
  (Utilities|Casting|CastToShip_BP OtherActor)
  (Default|CallPizzaAchievement))

(event EventBeginPlay
  (|CallParentFunction))

(event EventActorBeginOverlap
  (params (OtherActor :type Actor%20Object%20Reference)))

(event EventTick
  (params (DeltaSeconds :type Float%20%28single-precision%29))
  (|CallParentFunction 0.0)
  (Transformation|AddRelativeRotation (Class|KismetMathLibrary|MakeRot 0.0 0.0 (Variables|Default|GetRotaionIntensity)) false))

(fn ConstructionScript
  (|CallParentFunction))