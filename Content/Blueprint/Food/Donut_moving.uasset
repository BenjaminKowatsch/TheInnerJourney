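; Donut food actor that moves back and forth around its spawn position, apparently as a floating "breathing" motion.
; BeginPlay stores the initial location, and Tick plays or reverses the Food_Movement timeline according to the Up flag.
; Timeline updates add the Breathing track to that start location with a swept relative-location move, and each finish flips Up to loop the motion.
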(event EventBeginPlay
  (Variables|Default|Setinitial%20Position (Transformation|GetActorLocation)))

(event EventActorBeginOverlap
  (params (OtherActor :type Actor%20Object%20Reference)))

(event EventTick
  (params (DeltaSeconds :type Float%20%28single-precision%29))
  (if (Variables|Default|GetUp)
    (bind _breathing (Timeline|Food_Movement Play)
      (:Update
        (Transformation|SetActorRelativeLocation (+ _breathing (Variables|Default|Getinitial%20Position)) true))
      (:Finished
        (Variables|Default|SetUp (not (Variables|Default|GetUp)))))
    (else
      (Timeline|Food_Movement Reverse))))

(fn ConstructionScript)