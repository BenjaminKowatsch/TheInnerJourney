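; Base weapon projectile Blueprint that damages ships and destroys itself on impact.
; A timeline started on BeginPlay scales the actor over time.
; Hits play an impact cue, then destroy the projectile, applying damage only when the other actor casts to Ship_BP.
; Taking any damage also destroys it after a brief delay with the same sound.
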(event EventBeginPlay
  ;[1 1 1] Scale Projectile
  (bind _size (Timeline|Timeline_0 Play)
    (:Update
      (Transformation|SetActorRelativeScale3D (* "1.000000,1.000000,1.000000" _size)))))

(event EventAnyDamage
  (params (Damage :type Float%20%28single-precision%29) (DamageType :type Damage%20Type%20Object%20Reference) (InstigatedBy :type Controller%20Object%20Reference) (DamageCauser :type Actor%20Object%20Reference))
  ;[1 1 1] Destroy on Recieving Damage
  (Utilities|FlowControl|Delay 0.05)
  (Audio|PlaySoundatLocation "/Game/Sound/VirusHit/Virustreffer04_Cue.Virustreffer04_Cue" (Transformation|GetWorldLocation (Variables|Default|GetSphere1)))
  (Actor|DestroyActor))

(event EventHit
  (params (MyComp :type Primitive%20Component%20Object%20Reference) (Other :type Actor%20Object%20Reference) (OtherComp :type Primitive%20Component%20Object%20Reference) (bSelfMoved :type Boolean) (HitLocation :type Vector :default "0, 0, 0") (HitNormal :type Vector :default "0, 0, 0") (NormalImpulse :type Vector :default "0, 0, 0") (Hit :type Hit%20Result%20Structure%20%28by%20ref%29))
  ;[1 1 1] Apply Damage to Hit Object
  (Audio|PlaySoundatLocation "/Game/Sound/VirusHit/Virustreffer04_Cue.Virustreffer04_Cue" HitLocation)
  (bind _asship_bp (Utilities|Casting|CastToShip_BP Other)
    (:then
      (Actor|DestroyActor)
      (Game|Damage|ApplyDamage _asship_bp (Variables|Default|GetDamage) 0 0))
    (:CastFailed
      (Actor|DestroyActor))))

(fn ConstructionScript)