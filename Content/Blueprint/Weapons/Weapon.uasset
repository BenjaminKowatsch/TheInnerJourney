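; Hitscan weapon for the player's ship (Ship_BP) with ammo that recharges on a Tick timer and updates the ship.
; Fire events line-trace from the camera along its forward vector, or optionally to the last aim point when the HUD (Croshair_Hud or HudBloodstream) is hidden.
; FirePawnMoreDamage flags a quadruple-damage shot with a different beam.
; FireWeapon draws beams from two cockpit sockets to the hit, adds sparks and sounds, and applies damage.
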(event Custom|FirePawnMoreDamage
  (bind _returnvalue (Game|GetPlayerCameraManager 0))
  (bind _returnvalue_2 (Game|GetPlayerController 0))
  (bind _damage (Variables|Default|GetDamage))
  (bind _returnvalue_3 (Transformation|GetActorLocation _returnvalue))
  (bind _returnvalue_4 (HUD|GetHUD _returnvalue_2))
  (Variables|Default|SetQuadDamage true)
  (bind _ascroshair_hud (Utilities|Casting|CastToCroshair_Hud _returnvalue_4)
    (:then
      (if (Variables|/Game/Blueprint/HUD/Croshair_Hud.Croshair_Hud_C|GetIsHidden _ascroshair_hud)
        (if (Variables|Default|GetShootOnLastValidPosition) :!label _label
          (if (> (Variables|Default|GetAmmo) 0) :!label _label_2
            (bind _outhit (Collision|LineTraceByChannel _returnvalue_3 (Variables|Default|GetEnd) "TraceTypeQuery1" false (stale Custom|FirePawn Ignore) "None"))
            ;[1 1 1] Call your Widget Function Here
            (bind _output_get (Variables|Default|SetAmmo (- (Variables|Default|GetAmmo) 1)))
            (Default|UpdateAmmo (Variables|Default|GetShip) _output_get)
            (if (Variables|Default|GetQuadDamage)
              ;[1 1 1] Fire Better Weapon
              (CallFunction|FireWeapon (.HitActor (Collision|BreakHitResult _outhit)) (* _damage 4.0) (.Location (Collision|BreakHitResult _outhit)) "/Game/Particles/Weapons/P_BeamU.P_BeamU")
              (Variables|Default|SetQuadDamage false)
              (else
                ;[1 1 1] Normal Fire
                (CallFunction|FireWeapon (.HitActor (Collision|BreakHitResult _outhit)) _damage (.Location (Collision|BreakHitResult _outhit)) "/Game/Particles/Weapons/P_Beam.P_Beam")))))
        (else
          (Variables|Default|SetEnd (+ _returnvalue_3 (* (Transformation|GetActorForwardVector _returnvalue) 5e+05)) :!label _label_3)
          (goto _label_2))))
    (:CastFailed
      (bind _ashud_bloodstream (Utilities|Casting|CastToHudBloodstream _returnvalue_4))
      (if (Variables|/Game/Blueprint/HUD/HudBloodstream.HudBloodstream_C|GetIsHidden _ashud_bloodstream)
        (goto _label)
        (else
          (goto _label_3))))))

(event Custom|FirePawn
  (params (Ignore :type Array%20of%20Actor%20Object%20References))
  (bind _returnvalue (Game|GetPlayerCameraManager 0))
  (bind _returnvalue_2 (Game|GetPlayerController 0))
  (bind _damage (Variables|Default|GetDamage))
  (bind _returnvalue_3 (Transformation|GetActorLocation _returnvalue))
  (bind _returnvalue_4 (HUD|GetHUD _returnvalue_2))
  (bind _ascroshair_hud (Utilities|Casting|CastToCroshair_Hud _returnvalue_4)
    (:then
      (if (Variables|/Game/Blueprint/HUD/Croshair_Hud.Croshair_Hud_C|GetIsHidden _ascroshair_hud)
        (if (Variables|Default|GetShootOnLastValidPosition) :!label _label
          (if (> (Variables|Default|GetAmmo) 0) :!label _label_2
            (bind _outhit (Collision|LineTraceByChannel _returnvalue_3 (Variables|Default|GetEnd) "TraceTypeQuery1" false Ignore "None"))
            ;[1 1 1] Call your Widget Function Here
            (bind _output_get (Variables|Default|SetAmmo (- (Variables|Default|GetAmmo) 1)))
            (Default|UpdateAmmo (Variables|Default|GetShip) _output_get)
            (if (Variables|Default|GetQuadDamage)
              ;[1 1 1] Fire Better Weapon
              (CallFunction|FireWeapon (.HitActor (Collision|BreakHitResult _outhit)) (* _damage 4.0) (.Location (Collision|BreakHitResult _outhit)) "/Game/Particles/Weapons/P_BeamU.P_BeamU")
              (Variables|Default|SetQuadDamage false)
              (else
                ;[1 1 1] Normal Fire
                (CallFunction|FireWeapon (.HitActor (Collision|BreakHitResult _outhit)) _damage (.Location (Collision|BreakHitResult _outhit)) "/Game/Particles/Weapons/P_Beam.P_Beam")))))
        (else
          (Variables|Default|SetEnd (+ _returnvalue_3 (* (Transformation|GetActorForwardVector _returnvalue) 5e+05)) :!label _label_3)
          (goto _label_2))))
    (:CastFailed
      (bind _ashud_bloodstream (Utilities|Casting|CastToHudBloodstream _returnvalue_4))
      (if (Variables|/Game/Blueprint/HUD/HudBloodstream.HudBloodstream_C|GetIsHidden _ashud_bloodstream)
        (goto _label)
        (else
          (goto _label_3))))))

(event EventBeginPlay
  ;[1 1 1] Get Ship Actor
  (bind _outactors (Actor|GetAllActorsOfClass "/Game/Blueprint/FreeFlight/Ship_BP.Ship_BP_C"))
  (Variables|Default|SetShip (Utilities|Array|Get(acopy) _outactors)))

(event EventTick
  (params (DeltaSeconds :type Float%20%28single-precision%29))
  ;[1 1 1] Charge Logic
  (bind _output_get (Variables|Default|SetTime (+ (Variables|Default|GetTime) DeltaSeconds)))
  (if (> _output_get (Variables|Default|GetRechargeTime))
    (Variables|Default|SetTime 0.0)
    (if (> (Variables|Default|GetMax%20Ammo) (Variables|Default|GetAmmo))
      ;;[1 1 1] Call your Widget Function Here
      (bind _output_get_2 (Variables|Default|SetAmmo (+ (Variables|Default|GetAmmo) (Variables|Default|GetAmmo%20Amount%20per%20Charge))))
      (Default|UpdateAmmo (Variables|Default|GetShip) _output_get_2))))

(fn ConstructionScript)

(fn FireWeapon
  (params (DamagedActor :type Actor%20Object%20Reference) (BaseDamage :type Float%20%28single-precision%29) (Hit%20Location :type Vector :default "0, 0, 0") (Particle%20Effect :type Particle%20System%20Object%20Reference) (WeaponSound :type Sound%20Base%20Object%20Reference) (Hit%20Sound :type Sound%20Base%20Object%20Reference))
  (bind _ship (Variables|Default|GetShip))
  (bind _cockpit_combined (Variables|/Game/Blueprint/FreeFlight/Ship_BP.Ship_BP_C|GetCockpit_Combined _ship))
  (bind _returnvalue (Transformation|GetSocketLocation _cockpit_combined "WS"))
  (bind _returnvalue_2 (Transformation|GetSocketLocation _cockpit_combined "WS2"))
  (bind _returnvalue_3 (Effects|SpawnEmitteratLocation Particle%20Effect _returnvalue "0,0.000000, 0"))
  (bind _returnvalue_4 (Effects|SpawnEmitteratLocation Particle%20Effect _returnvalue_2 "0,0.000000, 0"))
  (Audio|PlaySoundatLocation WeaponSound _returnvalue)
  (Audio|PlaySoundatLocation WeaponSound _returnvalue_2)
  (Class|ParticleSystemComponent|SetBeamTargetPoint _returnvalue_3 0 Hit%20Location)
  (Effects|SpawnEmitteratLocation "/Game/Particles/Weapons/P_Sparks.P_Sparks" Hit%20Location)
  (Audio|PlaySoundatLocation Hit%20Sound Hit%20Location)
  (Game|Damage|ApplyDamage DamagedActor BaseDamage 0 0))