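; WeaponTestPawnLineTrace is a test hitscan weapon pawn that fires through a FirePawn event.
; Firing prints a debug message and line-traces on the Visibility channel from its Sphere component along the player camera's forward vector, with debug drawing.
; It spawns a test particle at the hit location and applies damage to the hit actor, without checking whether the trace hit.
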(event Custom|FirePawn
  (bind _sphere (Variables|Default|GetSphere))
  (bind _returnvalue (Transformation|GetWorldLocation _sphere))
  (Development|PrintString "Pew")
  (bind _outhit (Collision|LineTraceByChannel _returnvalue (+ _returnvalue (* (Transformation|GetActorForwardVector (Game|GetPlayerCameraManager 0)) 5e+03)) "TraceTypeQuery1" false 0 "ForDuration"))
  (Effects|SpawnEmitteratLocation "/Game/Particles/Weapons/TestParticle.TestParticle" (.Location (Collision|BreakHitResult _outhit)))
  (Game|Damage|ApplyDamage (.HitActor (Collision|BreakHitResult _outhit)) (Variables|Default|GetDamage) 0 0))

(fn ConstructionScript)