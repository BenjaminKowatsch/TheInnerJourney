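; StomachProjectile is a weapon projectile that damages the Ship_BP actor it hits.
; On BeginPlay a timeline drives its scale, and a short delay arms its overlap trigger.
; Once armed, any sphere overlap plays a virus hit sound and destroys the projectile, applying damage only to a Ship_BP.
; Taking any damage also destroys it with the same sound after a brief delay.
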(event OnComponentBeginOverlap(Sphere)
  (params (OtherActor :type Actor%20Object%20Reference) (OtherComp :type Primitive%20Component%20Object%20Reference) (OtherBodyIndex :type Integer) (bFromSweep :type Boolean) (SweepResult :type Hit%20Result%20Structure%20%28by%20ref%29))
  (if (Variables|Default|GetEnableTrigger)
    (Audio|PlaySoundatLocation "/Game/Sound/VirusHit/Virustreffer04_Cue.Virustreffer04_Cue" (Transformation|GetActorLocation))
    (bind _asship_bp (Utilities|Casting|CastToShip_BP OtherActor)
      (:then
        (Actor|DestroyActor)
        (Game|Damage|ApplyDamage _asship_bp (Variables|Default|GetDamage) 0 0))
      (:CastFailed
        (Actor|DestroyActor)))))

(event EventBeginPlay
  (Utilities|FlowControl|Sequence
    (:then_0
      (bind _size (Timeline|Timeline_0 Play)
        (:Update
          (Transformation|SetActorRelativeScale3D (* "3.000000,3.000000,3.000000" _size)))))
    (:then_1
      (Utilities|FlowControl|DoOnce false
        (:Completed
          (Utilities|FlowControl|Delay 0.5)
          (Variables|Default|SetEnableTrigger true))))))

(event EventAnyDamage
  (params (Damage :type Float%20%28single-precision%29) (DamageType :type Damage%20Type%20Object%20Reference) (InstigatedBy :type Controller%20Object%20Reference) (DamageCauser :type Actor%20Object%20Reference))
  (Utilities|FlowControl|Delay 0.05)
  (Audio|PlaySoundatLocation "/Game/Sound/VirusHit/Virustreffer04_Cue.Virustreffer04_Cue" (Transformation|GetWorldLocation (Variables|Default|GetSphere1)))
  (Actor|DestroyActor))

(fn ConstructionScript)