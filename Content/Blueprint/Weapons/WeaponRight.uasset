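; Right-hand hitscan weapon Blueprint that damages whatever the player is aiming at.
; FirePawn runs a visibility line trace along the camera's forward vector, skipping the passed-in actors, then applies damage to the hit actor with an impact effect.
; QuadDamage switches the shot from a laser particle aimed by a vector parameter to a beam ending at the hit point and quadruples the damage.
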(event Custom|FirePawn
  (params (Ignore :type Array%20of%20Actor%20Object%20References))
  (bind _returnvalue (Game|GetPlayerCameraManager 0))
  (bind _returnvalue_2 (Transformation|GetActorLocation))
  (bind _damage (Variables|Default|GetDamage))
  (bind _returnvalue_3 (Transformation|GetActorLocation _returnvalue))
  (bind _returnvalue_4 (Transformation|GetActorForwardVector _returnvalue))
  (bind _returnvalue_5 (* _returnvalue_4 5e+05))
  (bind _returnvalue_6 (+ _returnvalue_3 _returnvalue_5))
  (Development|PrintString "Right" true true "(R=1.000000,G=0.000000,B=0.012087,A=1.000000)")
  (bind (_outhit _returnvalue_7) (Collision|LineTraceByChannel _returnvalue_3 _returnvalue_6 "TraceTypeQuery1" false Ignore "None"))
  (if (Variables|Default|GetQuadDamage)
    (bind _returnvalue_8 (Effects|SpawnEmitteratLocation "/Game/Particles/Weapons/Beam.Beam" _returnvalue_2))
    (Class|ParticleSystemComponent|SetBeamTargetPoint _returnvalue_8 0 (.Location (Collision|BreakHitResult _outhit)))
    (Development|PrintString "Activated")
    (Effects|SpawnEmitteratLocation "/Game/Particles/Weapons/P_Steam_Lit.P_Steam_Lit" (.Location (Collision|BreakHitResult _outhit)))
    (Game|Damage|ApplyDamage (.HitActor (Collision|BreakHitResult _outhit)) (* _damage 4.0) 0 0)
    (else
      (bind _returnvalue_9 (Effects|SpawnEmitteratLocation "/Game/Particles/Weapons/P_Laser.P_Laser" _returnvalue_2))
      (Effects|Components|ParticleSystem|SetVectorParameter _returnvalue_9 "target" (* (Class|KismetMathLibrary|GetDirectionVector _returnvalue_2 (Math|Vector|SelectVector (.Location (Collision|BreakHitResult _outhit)) _returnvalue_6 _returnvalue_7)) 1e+05))
      (Effects|SpawnEmitteratLocation "/Game/Particles/Weapons/P_Steam_Lit.P_Steam_Lit" (.Location (Collision|BreakHitResult _outhit)) "0.000000, 0, 0")
      (Game|Damage|ApplyDamage (.HitActor (Collision|BreakHitResult _outhit)) _damage 0 0))))

(fn ConstructionScript)