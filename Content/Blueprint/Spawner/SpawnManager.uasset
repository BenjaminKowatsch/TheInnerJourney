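; Wave spawner actor that spawns enemy waves at the level's Spawnpoint actors until the last wave is finished.
; After a start delay it gathers all spawnpoints, then on Tick counts living enemies and, when none remain, starts the next delayed wave through a DoOnce gate.
; Each spawnpoint, up to a per-wave cap, spawns a random ground or air unit; ground units attach, bacteriophages receive waypoints.
; In brain levels, certain enemies become brain variants with overridden attack range.
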(event EventBeginPlay
  ;[1 1 1] Get All Spawnpoints in level
  (Utilities|FlowControl|Delay (Variables|Default|GetstartDelay))
  (bind _outactors (Actor|GetAllActorsOfClass "/Game/Blueprint/Spawner/Spawnpoint.Spawnpoint_C"))
  (Variables|Default|SetSpawnpoints _outactors)
  (Actor|Tick|SetActorTickEnabled true))

(event EventActorBeginOverlap
  (params (OtherActor :type Actor%20Object%20Reference)))

(event EventTick
  (params (DeltaSeconds :type Float%20%28single-precision%29))
  ;[1 1 1] If all spawned units are dead
  (bind _numberenemy (CallFunction|GetLivingActorNumber))
  (if (== _numberenemy 0)
    ;[1 1 1] start next wave, unless we are finished with last wave
    (Utilities|FlowControl|DoOnce false :!label _label
      (:Completed
        (bind _output_get (Variables|Default|SetcurrentWaveNumber (+ (Variables|Default|GetcurrentWaveNumber) 1)))
        (if (<= _output_get (Variables|Default|GetMaxWaveNumvber))
          (Utilities|FlowControl|Delay (Variables|Default|GetEnemySpawnDelay))
          (CallFunction|SpawnEnemies (Variables|Default|GetSpawnpoints))
          (for _array_element (Variables|Default|GetcurrentEnemies)
            _)
          (goto _label Reset)
          (else
            (Variables|Default|SetlastWaveFinished true)))))))

(fn ConstructionScript)

(fn SpawnEnemies
  (params (Spawnpoints :type Array%20of%20Spawnpoint%20Object%20References))
  (bind _spawnableunitsair (Variables|Default|GetSpawnableUnitsAir))
  (bind _spawnableunitsground (Variables|Default|GetSpawnableUnitsGround))
  ;[1 1 1] Iterate over each Spawnpoint
  (bind (_array_element _array_index) (Utilities|Array|ForEachLoopwithBreak Spawnpoints :!label _label)
    (:LoopBody
      (if (< _array_index (Variables|Default|GetMax%20Enemies%20per%20Wave))
        (bind _output_get (LocalVariables|SetcurrentSpawnpoint _array_element))
        ;[1 1 1] Getting Location From Spawnpoint
        (LocalVariables|SetcurrentSpawnTransform (Transformation|GetActorTransform _output_get))
        ;[1 1 1] Check For Spawnpoint Type
        (if (Variables|/Game/Blueprint/Spawner/Spawnpoint.Spawnpoint_C|GetGroundBool _output_get)
          ;[1 1 1] Spawn Random Ground Unit (gets attached to its spawnpoint
          (bind _returnvalue (Game|SpawnActorfromClass (Utilities|Array|Get(acopy) _spawnableunitsground (Math|Random|RandomIntegerinRange 0 (- (Utilities|Array|Length _spawnableunitsground) 1))) (LocalVariables|GetcurrentSpawnTransform) false 0))
          (Class|Actor|AttachRootComponenttoActor _returnvalue (LocalVariables|GetcurrentSpawnpoint) "None" "SnapToTarget" true)
          ;[1 1 1] Add Enemy to Current Enemies
          (Utilities|Array|Add (Variables|Default|GetcurrentEnemies) _returnvalue)
          ;[1 1 1] Make Enemy into Brain Enemy if in Brain Level ( Tobi)
          (if (Variables|Default|GetBrainLevel)
            (bind _asbot_turret_enemy_character (Utilities|Casting|CastToBotTurretEnemyCharacter _returnvalue))
            (Default|MakeBrainEnemy _asbot_turret_enemy_character)
            (Variables|/Game/Blueprint/Enemies/BotTurretEnemyCharacter.BotTurretEnemyCharacter_C|SetAttackRange _asbot_turret_enemy_character (Variables|Default|GetAttack%20Range%20of%20StandingTurret)))
          (else
            ;[1 1 1] Spawn Random Air Unit
            (bind _returnvalue_2 (Game|SpawnActorfromClass (Utilities|Array|Get(acopy) _spawnableunitsair (Math|Random|RandomIntegerinRange 0 (- (Utilities|Array|Length _spawnableunitsair) 1))) (LocalVariables|GetcurrentSpawnTransform) false 0))
            ;[1 1 1] Add Enemy to Current Enemies
            (Utilities|Array|Add (Variables|Default|GetcurrentEnemies) _returnvalue_2)
            ;[1 1 1] Check If Spawned Object is Bacteriophage
            (if (or (== (Utilities|GetClass _returnvalue_2) "/Game/Blueprint/Enemies/BotFlyingTurretEnemyCharacter.BotFlyingTurretEnemyCharacter_C") (== (Utilities|GetClass _returnvalue_2) "/Game/Blueprint/Enemies/BotBacteriophageCharacter.BotBacteriophageCharacter_C"))
              (bind _asbot_bacteriophage_character (Utilities|Casting|CastToBotBacteriophageCharacter _returnvalue_2))
              ;[1 1 1] Make Enemy into Brain Enemy if in Brain Level ( Tobi)
              (if (Variables|Default|GetBrainLevel)
                (Default|MakeBrainEnemy _asbot_bacteriophage_character)
                (Variables|/Game/Blueprint/Enemies/BotBacteriophageCharacter.BotBacteriophageCharacter_C|SetAttackRange _asbot_bacteriophage_character (Variables|Default|GetAttackRange%20of%20Poison%20Bots)))
              ;[1 1 1] Add Waypoints To Bacteriophage
              (for _array_element_2 (Variables|/Game/Blueprint/Spawner/Spawnpoint.Spawnpoint_C|GetWaypoints (LocalVariables|GetcurrentSpawnpoint))
                (Default|AddWaypoint _asbot_bacteriophage_character _array_element_2)))))
        (else
          (goto _label Break))))))

(fn GetLivingActorNumber
  (LocalVariables|SetEnemyNumber 0) ; Set to 0 in the beginning
  (for _array_element (Variables|Default|GetcurrentEnemies)
    (if (Utilities|IsValid _array_element)
      (LocalVariables|SetEnemyNumber (+ (LocalVariables|GetEnemyNumber) 1))
      (else
        (Utilities|Array|RemoveItem (Variables|Default|GetcurrentEnemies) _array_element))))
  ;[1 1 1] return EnemyNumber
  (return (LocalVariables|GetEnemyNumber)))