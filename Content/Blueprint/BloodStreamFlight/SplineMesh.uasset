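; Spline path actor for the bloodstream flight that hands an overlapping Ship_BP to its spline.
; The construction script stores world location and rotation of the spline's first and last points in SplinePoints and SplineRotators.
; It then adds one spline mesh per segment under Scene, shaped by neighboring points' local locations and tangents.
; When a Ship_BP begins overlapping the Box, it calls AttachTo on that ship with the Spline.
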(event OnComponentBeginOverlap(Box)
  (params (OtherActor :type Actor%20Object%20Reference) (OtherComp :type Primitive%20Component%20Object%20Reference) (OtherBodyIndex :type Integer) (bFromSweep :type Boolean) (SweepResult :type Hit%20Result%20Structure%20%28by%20ref%29))
  (bind _asship_bp (Utilities|Casting|CastToShip_BP OtherActor))
  (Default|Attachto _asship_bp (Variables|Default|GetSpline)))

(event EventBeginPlay)

(event EventActorBeginOverlap
  (params (OtherActor :type Actor%20Object%20Reference)))

(event EventTick
  (params (DeltaSeconds :type Float%20%28single-precision%29)))

(fn ConstructionScript
  (bind _spline_rotators (Variables|Default|GetSpline%20Rotators))
  (bind _spline (Variables|Default|GetSpline))
  (bind _splinepoints (Variables|Default|GetSplinePoints))
  (bind _spline_2 (Variables|Default|GetSpline))
  (bind _returnvalue (Class|SplineComponent|GetNumSplinePoints _spline))
  (bind _returnvalue_2 (Spline|GetDistanceAlongSplineatSplinePoint _spline_2 0))
  (bind _returnvalue_3 (- _returnvalue 1))
  (bind _returnvalue_4 (Spline|GetDistanceAlongSplineatSplinePoint _spline_2 _returnvalue_3))
  (Utilities|Array|SetArrayElem _splinepoints 0 (Class|SplineComponent|GetWorldLocationatDistanceAlongSpline _spline_2 _returnvalue_2))
  (Utilities|Array|SetArrayElem _spline_rotators 0 (Class|SplineComponent|GetWorldRotationatDistanceAlongSpline _returnvalue_2))
  (Utilities|Array|SetArrayElem _splinepoints 1 (Class|SplineComponent|GetWorldLocationatDistanceAlongSpline _spline_2 _returnvalue_4))
  (Utilities|Array|SetArrayElem _spline_rotators 1 (Class|SplineComponent|GetWorldRotationatDistanceAlongSpline _returnvalue_4))
  (for _index (range 0 (- _returnvalue 2))
    (bind _returnvalue_5 (AddComponent|AddSplineMeshComponent true))
    (Class|SceneComponent|Attachto _returnvalue_5 (Variables|Default|GetScene) "None" "KeepRelativeOffset" true)
    (SplineMesh|SetStartandEnd _returnvalue_5 (.LocalLocation (Class|SplineComponent|GetLocalLocationandTangentatSplinePoint _spline _index)) (.LocalTangent (Class|SplineComponent|GetLocalLocationandTangentatSplinePoint _spline _index)) (.LocalLocation (Class|SplineComponent|GetLocalLocationandTangentatSplinePoint _spline (+ _index 1))) (.LocalTangent (Class|SplineComponent|GetLocalLocationandTangentatSplinePoint _spline (+ _index 1))) :!class /Script/Engine.SplineMeshComponent)))