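; Protein supply actor for the blood stream flight game that acts as a depleting resource gauge tied to the player's ship.
; Each tick runs a loop that waits a set delay, lowers the current supply by a fixed amount and refreshes a widget component's progress bar with the remaining fraction.
; When the supply runs out, it destroys the referenced ship actor.
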(event Custom|UpdateWidget
  ;[1 1 1] UpdateWidget
  (bind _asproteinsupply (Utilities|Casting|CastToProteinsupply (UserInterface|GetUserWidgetObject (Variables|Default|GetWidget))))
  (Progress|SetPercent (Variables|/Game/Blueprint/HUD/Proteinsupply.Proteinsupply_C|GetProgressBar_83 _asproteinsupply) (/ (Variables|Default|GetCurrentSupply) (Variables|Default|GetMaxSupply))))

(event EventTick
  (params (DeltaSeconds :type Float%20%28single-precision%29))
  ;[1 1 1] GameLoop
  (if (> (Variables|Default|GetCurrentSupply) 0.0) :!label _label
    (Utilities|FlowControl|Delay (Variables|Default|GetDecreaseDelay))
    (Variables|Default|SetCurrentSupply (- (Variables|Default|GetCurrentSupply) (Variables|Default|GetDecreaseValue)))
    (CallFunction|UpdateWidget)
    (goto _label)
    (else
      (Actor|DestroyActor (Variables|Default|GetShipReference)))))

(fn ConstructionScript)