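; Bacteriophage enemy for the blood stream flight game that chases the player when it spots them.
; Pawn sensing filters for the flight pawn, then sends the AI controller on a simple move to the player's location at that moment.
; An UpdateRotation event smoothly turns the skeletal mesh along the player-to-mesh look-at direction, but its Tick-style call is disconnected, so it never runs.
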(event OnSeePawn(PawnSensing)
  (params (Pawn :type Pawn%20Object%20Reference))
  (Utilities|Casting|CastToPlainFlightPawn Pawn)
  (bind _asaicontroller (Utilities|Casting|CastToAIController (Pawn|GetController)))
  (AI|Navigation|SimpleMovetoLocation _asaicontroller (Transformation|GetActorLocation (Game|Player|GetPlayerPawn 0))))

(event Custom|UpdateRotation
  (bind _returnvalue (Game|Player|GetPlayerPawn 0))
  (bind _skeletalmesh (Variables|Default|GetSkeletalMesh))
  (bind _returnvalue_2 (Transformation|GetActorLocation _returnvalue))
  (bind _returnvalue_3 (Transformation|GetWorldLocation _skeletalmesh))
  (bind _returnvalue_4 (Math|Rotator|FindLookatRotation _returnvalue_2 _returnvalue_3))
  (bind (_pitch _yaw _roll) (Class|KismetMathLibrary|BreakRot _returnvalue_4))
  (Transformation|SetWorldRotation (Variables|Default|GetSkeletalMesh) (Math|Interpolation|RInterpTo (Transformation|GetWorldRotation (Variables|Default|GetSkeletalMesh)) (Class|KismetMathLibrary|MakeRot _pitch _yaw _roll) (Variables|Default|GetDeltaTime) (Variables|Default|GetRotationSpeed)) false))

(event EventTick
  (params (DeltaSeconds :type Float%20%28single-precision%29)))

(fn ConstructionScript)