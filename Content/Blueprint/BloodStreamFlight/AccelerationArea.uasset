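; Box trigger area in the BloodStreamFlight game that speeds up the player ship (Ship_BP) on entry and slows it on exit.
; Begin overlap sets a target MaxSpeedOffset above SteadySpeed; end overlap sets one the same amount below the current value.
; Delay loops step SteadySpeed by Acceleration or Deceleration roughly each frame, unscaled by delta time.
; Both loops share the SpeedOffset variable, so leaving mid-ramp retargets the acceleration loop.
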(event OnComponentBeginOverlap(Box)
  (params (OtherActor :type Actor%20Object%20Reference) (OtherComp :type Primitive%20Component%20Object%20Reference) (OtherBodyIndex :type Integer) (bFromSweep :type Boolean) (SweepResult :type Hit%20Result%20Structure%20%28by%20ref%29))
  (bind _asship_bp (Utilities|Casting|CastToShip_BP OtherActor))
  (Variables|Default|SetSpeedOffset (+ (Variables|/Game/Blueprint/FreeFlight/Ship_BP.Ship_BP_C|GetSteady%20Speed _asship_bp) (Variables|Default|GetMaxSpeedOffset)))
  (if (< (Variables|/Game/Blueprint/FreeFlight/Ship_BP.Ship_BP_C|GetSteady%20Speed _asship_bp) (Variables|Default|GetSpeedOffset)) :!label _label
    (Variables|/Game/Blueprint/FreeFlight/Ship_BP.Ship_BP_C|SetSteady%20Speed _asship_bp (+ (Variables|Default|GetAcceleration) (Variables|/Game/Blueprint/FreeFlight/Ship_BP.Ship_BP_C|GetSteady%20Speed _asship_bp)))
    (Utilities|FlowControl|Delay (Utilities|Time|GetWorldDeltaSeconds))
    (goto _label)))

(event OnComponentEndOverlap(Box)
  (params (OtherActor :type Actor%20Object%20Reference) (OtherComp :type Primitive%20Component%20Object%20Reference) (OtherBodyIndex :type Integer))
  (bind _asship_bp (Utilities|Casting|CastToShip_BP OtherActor))
  (Variables|Default|SetSpeedOffset (- (Variables|/Game/Blueprint/FreeFlight/Ship_BP.Ship_BP_C|GetSteady%20Speed _asship_bp) (Variables|Default|GetMaxSpeedOffset)))
  (if (> (Variables|/Game/Blueprint/FreeFlight/Ship_BP.Ship_BP_C|GetSteady%20Speed _asship_bp) (Variables|Default|GetSpeedOffset)) :!label _label
    (Variables|/Game/Blueprint/FreeFlight/Ship_BP.Ship_BP_C|SetSteady%20Speed _asship_bp (- (Variables|/Game/Blueprint/FreeFlight/Ship_BP.Ship_BP_C|GetSteady%20Speed _asship_bp) (Variables|Default|GetDeceleration)))
    (Utilities|FlowControl|Delay (Utilities|Time|GetWorldDeltaSeconds))
    (goto _label)))

(fn ConstructionScript)