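; Player-controlled free-flight pawn with VR headset reset and a laser weapon.
; Movement axes set a normalized acceleration that Tick integrates into velocity, decelerating without input and moving by a speed-clamped, swept local offset.
; Look axes add relative rotation, and hits reverse velocity at reduced strength.
; G spawns a Laser_Weapon if none is valid, and the Shoot axis fires it along the camera's forward vector.
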(event EventHit
  (params (MyComp :type Primitive%20Component%20Object%20Reference) (Other :type Actor%20Object%20Reference) (OtherComp :type Primitive%20Component%20Object%20Reference) (bSelfMoved :type Boolean) (HitLocation :type Vector :default "0, 0, 0") (HitNormal :type Vector :default "0, 0, 0") (NormalImpulse :type Vector :default "0, 0, 0") (Hit :type Hit%20Result%20Structure%20%28by%20ref%29))
  ;[1 1 1] Collision
  (Variables|Default|SetVelocity (* (Variables|Default|GetVelocity) -0.2)))

(event EventTick
  (params (DeltaSeconds :type Float%20%28single-precision%29))
  (bind _acceleration (Variables|Default|GetAcceleration))
  ;[1 1 1] Update Positions
  (bind _output_get (Variables|Default|SetVelocity (+ (* (Math|Vector|SelectVector (* (Math|Vector|Normalize (* (Variables|Default|GetVelocity) -1.0)) (Variables|Default|GetDecelerationFactor)) _acceleration (and (== (Math|Vector|VectorLengthSquared _acceleration) 0.0) (!= (Math|Vector|VectorLengthSquared (Variables|Default|GetVelocity)) 0.0))) DeltaSeconds) (Variables|Default|GetVelocity))))
  (Transformation|AddLocalOffset (* (Math|Vector|ClampVectorSize _output_get (Variables|Default|GetMinVelocity) (Variables|Default|GetMaxVelocity)) DeltaSeconds) true))

(event Input|ActionEvents|InputActionResetHMD
  ;[1 1 1] Reset HMD Rotation
  (:Pressed
    (Class|HeadMountedDisplayFunctionLibrary|ResetOrientationandPosition 0.0 "OrientationAndPosition")))

(event Input|AxisEvents|InputAxisLookRight
  (params (AxisValue :type Float%20%28single-precision%29))
  ;[1 1 1] Camera Rotation
  (Transformation|AddRelativeRotation (Class|KismetMathLibrary|MakeRot (stale Input|AxisEvents|InputAxisLookUp AxisValue) AxisValue 0.0) false))

(event Input|AxisEvents|InputAxisMoveUp
  (params (AxisValue :type Float%20%28single-precision%29))
  ;[1 1 1] Update Acceleration
  (Variables|Default|SetAcceleration (* (Math|Vector|Normalize (Math|Vector|MakeVector (stale Input|AxisEvents|InputAxisMoveForward AxisValue) (stale Input|AxisEvents|InputAxisMoveRight AxisValue) AxisValue)) (Variables|Default|GetAccelerationFactor))))

(event Input|AxisEvents|InputAxisMoveRight
  (params (AxisValue :type Float%20%28single-precision%29))
  ;[1 1 1] Update Acceleration
  (Variables|Default|SetAcceleration (* (Math|Vector|Normalize (Math|Vector|MakeVector (stale Input|AxisEvents|InputAxisMoveForward AxisValue) AxisValue (stale Input|AxisEvents|InputAxisMoveUp AxisValue))) (Variables|Default|GetAccelerationFactor))))

(event Input|AxisEvents|InputAxisShoot
  (params (AxisValue :type Float%20%28single-precision%29))
  (bind _returnvalue (Game|GetPlayerCameraManager 0))
  (bind _currentweapon (Variables|Default|GetCurrentWeapon))
  ;[1 1 1] Shoot
  (if (!= AxisValue 0.0)
    (Utilities|IsValid _currentweapon
      (:Is%20Valid
        (Default|FireEvent _currentweapon (+ (Transformation|GetActorLocation _returnvalue) "200.000000,0.000000,-50.000000") (* (Transformation|GetActorForwardVector _returnvalue) 5e+03))))))

(event Input|AxisEvents|InputAxisMoveForward
  (params (AxisValue :type Float%20%28single-precision%29))
  ;[1 1 1] Update Acceleration
  (Variables|Default|SetAcceleration (* (Math|Vector|Normalize (Math|Vector|MakeVector AxisValue (stale Input|AxisEvents|InputAxisMoveRight AxisValue) (stale Input|AxisEvents|InputAxisMoveUp AxisValue))) (Variables|Default|GetAccelerationFactor))))

(event Input|AxisEvents|InputAxisLookUp
  (params (AxisValue :type Float%20%28single-precision%29))
  ;[1 1 1] Camera Rotation
  (Transformation|AddRelativeRotation (Class|KismetMathLibrary|MakeRot AxisValue (stale Input|AxisEvents|InputAxisLookRight AxisValue) 0.0) false))

(event Input|KeyboardEvents|G
  ;[1 1 1] Set CurrentWeapon if it's not valid
  (:Pressed
    (Utilities|IsValid (Variables|Default|GetCurrentWeapon)
      (:Is%20Not%20Valid
        (bind _returnvalue (Game|SpawnActorfromClass "/Game/Blueprint/BloodStreamFlight/Laser_Weapon.Laser_Weapon_C" (Transformation|GetActorTransform) false 0))
        (Variables|Default|SetCurrentWeapon _returnvalue)))))

(fn ConstructionScript)