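; Protein supply meter for the bloodstream flight section that drains over time and damages the ship when empty.
; While the ship is in the bloodstream, a Tick-driven Delay loop lowers the supply and updates a widget progress bar with the remaining fraction.
; Once supply is depleted, delayed checks apply low-supply damage to the referenced ship.
; BeginPlay also calls SetHiddenInGame on the ship reference.
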(event Custom|UpdateWidget
  ;[1 1 1] UpdateWidget
  (bind _asproteinsupply (Utilities|Casting|CastToProteinsupply (UserInterface|GetUserWidgetObject)))
  (Progress|SetPercent (Variables|/Game/Blueprint/HUD/Proteinsupply.Proteinsupply_C|GetProgressBar_83 _asproteinsupply) (/ (Variables|Default|GetCurrentSupply) (Variables|Default|GetMaxSupply))))

(event EventTick
  (params (DeltaSeconds :type Float%20%28single-precision%29))
  ;[1 1 1] GameLoop
  (if (Variables|/Game/Blueprint/FreeFlight/Ship_BP.Ship_BP_C|GetinBloodstream (Variables|Default|GetShipReference))
    (Utilities|FlowControl|Delay (Variables|Default|GetDecreaseDelay) :!label _label)
    (if (> (Variables|Default|GetCurrentSupply) 0.0)
      (Variables|Default|SetCurrentSupply (- (Variables|Default|GetCurrentSupply) (Variables|Default|GetDecreaseValue)))
      (CallFunction|UpdateWidget)
      (goto _label)
      (else
        (Game|Damage|ApplyDamage (Variables|Default|GetShipReference) (Variables|Default|GetLowSupplyDamage) 0 0)))))

(event EventBeginPlay
  ;[1 1 1] GameLoop
  (Development|SetHiddeninGame (Variables|Default|GetShipReference) true false))

(fn ConstructionScript)