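; Ship Blueprint that moves itself along its local forward axis at a speed controlled by the Accelerate input axis.
; The axis handler adds scaled acceleration to the current forward speed, or decelerates at half that rate without input, clamped between minimum and maximum speeds.
; Tick applies that speed as a frame-rate-independent local offset without sweeping for collisions.
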(event EventTick
  (params (DeltaSeconds :type Float%20%28single-precision%29))
  ;[1 1 1] Apply Current Forward Speed
  (Transformation|AddActorLocalOffset (Math|Vector|MakeVector (* DeltaSeconds (Variables|Default|GetCurrentForwardSpeed)) 0.0 0.0) false))

(event Input|AxisEvents|InputAxisAccelerate
  (params (AxisValue :type Float%20%28single-precision%29))
  (bind _acceleration (Variables|Default|GetAcceleration))
  ;[1 1 1] Set Forward Movement Speed
  (Variables|Default|SetCurrentForwardSpeed (Math|Float|Clamp(Float) (+ (Variables|Default|GetCurrentForwardSpeed) (* (Math|Float|SelectFloat (* AxisValue _acceleration) (* _acceleration -0.5) (!= AxisValue 0.0)) (Utilities|Time|GetWorldDeltaSeconds))) (Variables|Default|GetMin%20Speed) (Variables|Default|GetMax%20Speed))))

(fn ConstructionScript)