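; Player-flown free-flight ship with HMD recentering and an attachable weapon.
; Axis inputs build clamped forward, pitch, yaw and roll speeds, braked by CalculateBreak without input; Tick applies them as local movement and rotation, and hits zero forward speed.
; Tick also traces from the camera and spawns a crosshair decal at the hit location.
; An overlapped WeaponTestPawn is shrunk, snapped to the cockpit's WS socket and fired through the Fire input.
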(event OnComponentHit(UFO)
  (params (OtherActor :type Actor%20Object%20Reference) (OtherComp :type Primitive%20Component%20Object%20Reference) (NormalImpulse :type Vector :default "0, 0, 0") (Hit :type Hit%20Result%20Structure%20%28by%20ref%29))
  ;[1 1 1] Collision
  (Variables|CurrentSpeedValues|SetCurrentSpeed 0.0))

(event EventActorBeginOverlap
  (params (OtherActor :type Actor%20Object%20Reference))
  ;[1 1 1] Add and use Weapon
  (bind _asweapon_test_pawn (Utilities|Casting|CastToWeaponTestPawn OtherActor))
  (Transformation|SetRelativeScale3D _asweapon_test_pawn "0.100000,0.100000,0.100000")
  (Class|Actor|AttachRootComponentto _asweapon_test_pawn (Variables|Default|GetCockpit_Combined) "WS" "SnapToTarget" true))

(event EventTick
  (params (DeltaSeconds :type Float%20%28single-precision%29))
  (bind _returnvalue (Game|GetPlayerCameraManager 0))
  (bind _returnvalue_2 (Utilities|Time|GetWorldDeltaSeconds))
  (bind _returnvalue_3 (Transformation|GetActorLocation _returnvalue))
  ;[1 1 1] Apply Current Speed
  (Transformation|AddActorLocalOffset (Math|Vector|MakeVector (* DeltaSeconds (Variables|CurrentSpeedValues|GetCurrentSpeed)) 0.0 0.0) true)
  (Transformation|AddActorLocalRotation (Class|KismetMathLibrary|MakeRot 0.0 (* _returnvalue_2 (Variables|CurrentSpeedValues|GetCurrent%20Yaw%20Speed)) (* _returnvalue_2 (Variables|CurrentSpeedValues|GetCurrent%20Roll%20Speed))) false)
  (Transformation|AddActorLocalRotation (Class|KismetMathLibrary|MakeRot (* (Utilities|Time|GetWorldDeltaSeconds) (Variables|CurrentSpeedValues|GetCurrent%20Pitch%20Speed)) 0.0 0.0) false)
  ;[1 1 1] Line Trace Crosair
  (bind _outhit (Collision|LineTraceByChannel _returnvalue_3 (+ _returnvalue_3 (* (Transformation|GetActorForwardVector _returnvalue) 5e+03)) "TraceTypeQuery1" false 0 "None"))
  (Rendering|Decal|SpawnDecalatLocation "/Game/Meshes/Ship/WingsSeat.WingsSeat" "10.000000,10.000000, 0" (.Location (Collision|BreakHitResult _outhit)) "-90.000000,0.000000,0.000000" (/ 1.0 (Utilities|Time|GetWorldDeltaSeconds))))

(event EventHit
  (params (MyComp :type Primitive%20Component%20Object%20Reference) (Other :type Actor%20Object%20Reference) (OtherComp :type Primitive%20Component%20Object%20Reference) (bSelfMoved :type Boolean) (HitLocation :type Vector :default "0, 0, 0") (HitNormal :type Vector :default "0, 0, 0") (NormalImpulse :type Vector :default "0, 0, 0") (Hit :type Hit%20Result%20Structure%20%28by%20ref%29))
  ;[1 1 1] Collision
  (Variables|CurrentSpeedValues|SetCurrentSpeed 0.0))

(event Input|ActionEvents|InputActionFire
  ;[1 1 1] Add and use Weapon
  (:Pressed
    (Default|FirePawn (stale EventActorBeginOverlap _asweapon_test_pawn))))

(event Input|ActionEvents|InputActionResetHMD
  ;[1 1 1] Reset HMD Rotation
  (:Pressed
    (Class|HeadMountedDisplayFunctionLibrary|ResetOrientationandPosition 0.0 "OrientationAndPosition")))

(event Input|AxisEvents|InputAxisYaw
  (params (AxisValue :type Float%20%28single-precision%29))
  (bind _max_yaw_speed (Variables|MaxSpeedValues|GetMax%20Yaw%20Speed))
  ;[1 1 1] Yaw right
  (Variables|CurrentSpeedValues|SetCurrent%20Yaw%20Speed (Math|Float|Clamp(Float) (- (Variables|CurrentSpeedValues|GetCurrent%20Yaw%20Speed) (* (Math|Float|SelectFloat (* AxisValue (Variables|AccelerationValues|GetYaw%20Acceleration)) (Class|ExtendedFunctions|CalculateBreak (* (Variables|CurrentSpeedValues|GetCurrent%20Yaw%20Speed) -1.0) (Variables|AccelerationValues|GetYaw%20Acceleration)) (!= AxisValue 0.0)) (Utilities|Time|GetWorldDeltaSeconds))) (* _max_yaw_speed -1.0) _max_yaw_speed)))

(event Input|AxisEvents|InputAxisAccelerate
  (params (AxisValue :type Float%20%28single-precision%29))
  (bind _max_speed (Variables|MaxSpeedValues|GetMax%20Speed))
  ;[1 1 1] Set Movement Speed
  (Variables|CurrentSpeedValues|SetCurrentSpeed (Math|Float|SelectFloat 0.0 (Math|Float|Clamp(Float) (+ (Variables|CurrentSpeedValues|GetCurrentSpeed) (* (Math|Float|SelectFloat (* AxisValue (Variables|AccelerationValues|GetAcceleration)) (Class|ExtendedFunctions|CalculateBreak (Variables|CurrentSpeedValues|GetCurrentSpeed) (Variables|"Physics"|GetResistance)) (!= AxisValue 0.0)) (Utilities|Time|GetWorldDeltaSeconds))) (* _max_speed -1.0) _max_speed) (Math|Float|InRange(Float) (Math|Float|Clamp(Float) (+ (Variables|CurrentSpeedValues|GetCurrentSpeed) (* (Math|Float|SelectFloat (* AxisValue (Variables|AccelerationValues|GetAcceleration)) (Class|ExtendedFunctions|CalculateBreak (Variables|CurrentSpeedValues|GetCurrentSpeed) (Variables|"Physics"|GetResistance)) (!= AxisValue 0.0)) (Utilities|Time|GetWorldDeltaSeconds))) (* _max_speed -1.0) _max_speed) -0.1 0.1))))

(event Input|AxisEvents|InputAxisPitch
  (params (AxisValue :type Float%20%28single-precision%29))
  (bind _max_pitch_speed (Variables|MaxSpeedValues|GetMax%20Pitch%20Speed))
  ;[1 1 1] Set Pitch Speed
  (Variables|CurrentSpeedValues|SetCurrent%20Pitch%20Speed (Math|Float|SelectFloat 0.0 (Math|Float|Clamp(Float) (+ (Variables|CurrentSpeedValues|GetCurrent%20Pitch%20Speed) (* (Math|Float|SelectFloat (* AxisValue (Variables|AccelerationValues|GetPitch%20Acceleration)) (Class|ExtendedFunctions|CalculateBreak (Variables|CurrentSpeedValues|GetCurrent%20Pitch%20Speed) (Variables|AccelerationValues|GetPitch%20Acceleration)) (!= AxisValue 0.0)) (Utilities|Time|GetWorldDeltaSeconds))) (* -1.0 _max_pitch_speed) _max_pitch_speed) (Math|Float|InRange(Float) (Math|Float|Clamp(Float) (+ (Variables|CurrentSpeedValues|GetCurrent%20Pitch%20Speed) (* (Math|Float|SelectFloat (* AxisValue (Variables|AccelerationValues|GetPitch%20Acceleration)) (Class|ExtendedFunctions|CalculateBreak (Variables|CurrentSpeedValues|GetCurrent%20Pitch%20Speed) (Variables|AccelerationValues|GetPitch%20Acceleration)) (!= AxisValue 0.0)) (Utilities|Time|GetWorldDeltaSeconds))) (* -1.0 _max_pitch_speed) _max_pitch_speed) -0.1 0.1))))

(event Input|AxisEvents|InputAxisRoll
  (params (AxisValue :type Float%20%28single-precision%29))
  (bind _max_roll_speed (Variables|MaxSpeedValues|GetMax%20Roll%20Speed))
  ;[1 1 1] Set Roll Speed
  (Variables|CurrentSpeedValues|SetCurrent%20Roll%20Speed (Math|Float|Clamp(Float) (- (Variables|CurrentSpeedValues|GetCurrent%20Roll%20Speed) (* (Math|Float|SelectFloat (* AxisValue (Variables|AccelerationValues|GetRoll%20Acceleration)) (Class|ExtendedFunctions|CalculateBreak (* (Variables|CurrentSpeedValues|GetCurrent%20Roll%20Speed) -1.0) (Variables|AccelerationValues|GetRoll%20Acceleration)) (!= AxisValue 0.0)) (Utilities|Time|GetWorldDeltaSeconds))) (* -1.0 _max_roll_speed) _max_roll_speed)))

(fn ConstructionScript)